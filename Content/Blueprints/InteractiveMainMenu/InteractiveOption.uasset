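; InteractiveOption is an in-world 3D menu option for an interactive main menu, shown as a text render with a capsule trigger.
; The construction script applies the configurable text, location, default size, color and optional font.
; A pawn overlapping the capsule recolors and resizes the text and enables the actor's input for the player controller; leaving restores the defaults and disables input.
; No selection action is implemented here.
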(event OnComponentBeginOverlap(Capsule)
  (params (OverlappedComponent :type Primitive%20Component%20Object%20Reference) (OtherActor :type Actor%20Object%20Reference) (OtherComp :type Primitive%20Component%20Object%20Reference) (OtherBodyIndex :type Integer) (bFromSweep :type Boolean) (SweepResult :type Hit%20Result%20Structure%20%28by%20ref%29))
  (Utilities|Casting|CastToPawn OtherActor)
  ;[1 1 1] Change Text Based on Overlap
  (Rendering|Components|TextRender|SetTextRenderColor (Variables|Default|GetOptionText) (Math|Conversions|ToColor(LinearColor) (Variables|Text|Color|GetColor)))
  (Rendering|Components|TextRender|SetWorldSize (Variables|Default|GetOptionText) (Variables|Text|Size|GetSize))
  (Input|EnableInput (Game|GetPlayerController (Variables|Player|GetPlayerIndex))))

(event OnComponentEndOverlap(Capsule)
  (params (OverlappedComponent :type Primitive%20Component%20Object%20Reference) (OtherActor :type Actor%20Object%20Reference) (OtherComp :type Primitive%20Component%20Object%20Reference) (OtherBodyIndex :type Integer))
  (Utilities|Casting|CastToPawn OtherActor)
  ;[1 1 1] Change Text Based on Overlap
  (Rendering|Components|TextRender|SetTextRenderColor (Variables|Default|GetOptionText) (Math|Conversions|ToColor(LinearColor) (Variables|Text|Color|GetDefaultColor)))
  (Rendering|Components|TextRender|SetWorldSize (Variables|Default|GetOptionText) (Variables|Text|Size|GetDefaultSize))
  (Input|DisableInput (Game|GetPlayerController (Variables|Player|GetPlayerIndex))))

(event EventBeginPlay)

(event Collision|EventActorBeginOverlap
  (params (OtherActor :type Actor%20Object%20Reference)))

(event EventTick
  (params (DeltaSeconds :type Float%20%28single-precision%29)))

(fn ConstructionScript
  ;[1 1 1] Set Default Text Look
  (Rendering|Components|TextRender|SetText (Variables|Default|GetOptionText) (Variables|Text|GetText))
  (Transformation|SetRelativeLocation (Variables|Default|GetOptionText) (Variables|Text|GetTextLocation) false false)
  (Rendering|Components|TextRender|SetWorldSize (Variables|Default|GetOptionText) (Variables|Text|Size|GetDefaultSize))
  (Rendering|Components|TextRender|SetTextRenderColor (Variables|Default|GetOptionText) (Math|Conversions|ToColor(LinearColor) (Variables|Text|Color|GetDefaultColor)))
  (Utilities|IsValid (Variables|Text|Font|GetFont)
    (:Is%20Valid
      (Class|TextRenderComponent|SetFont (Variables|Default|GetOptionText) (Variables|Text|Font|GetFont)))))