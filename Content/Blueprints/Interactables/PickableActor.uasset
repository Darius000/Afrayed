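; Interactable world item that the Pinn_Bp character can pick up into its inventory.
; Sphere overlap shows a pickup prompt or "Inventory Full" notice based on inventory space, and removes it on exit.
; PickUp relies on a passed-in can-add flag, then adds the item to the inventory, calls InteractWith and destroys the actor.
; The construction script sets the billboard sprite from the item's Icon.
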(event OnComponentEndOverlap(Sphere)
  (params (OverlappedComponent :type Primitive%20Component%20Object%20Reference) (OtherActor :type Actor%20Object%20Reference) (OtherComp :type Primitive%20Component%20Object%20Reference) (OtherBodyIndex :type Integer))
  (Utilities|Casting|CastToPinn_Bp OtherActor)
  (Widget|RemovefromParent (Variables|Default|GetNotification)))

(event OnComponentBeginOverlap(Sphere)
  (params (OverlappedComponent :type Primitive%20Component%20Object%20Reference) (OtherActor :type Actor%20Object%20Reference) (OtherComp :type Primitive%20Component%20Object%20Reference) (OtherBodyIndex :type Integer) (bFromSweep :type Boolean) (SweepResult :type Hit%20Result%20Structure%20%28by%20ref%29))
  (bind _aspinn_bp (Utilities|Casting|CastToPinn_Bp OtherActor))
  (if (Default|HaveSpace (Variables|/Game/PinnBP/Pinn_Bp.Pinn_Bp_C|GetInventory _aspinn_bp))
    (bind _returnvalue (UserInterface|CreateWidget "/Game/UI/PickUpNotification.PickUpNotification_C" 0 "Press 'E' to Pick Up"))
    (Variables|Default|SetNotification _returnvalue)
    (else
      (bind _returnvalue_2 (UserInterface|CreateWidget "/Game/UI/PickUpNotification.PickUpNotification_C" 0 "Inventory Full"))
      (Variables|Default|SetNotification _returnvalue_2)))
  (UserInterface|Viewport|AddtoViewport (Variables|Default|GetNotification) 3))

(event EventBeginPlay)

(event Collision|EventActorBeginOverlap
  (params (OtherActor :type Actor%20Object%20Reference)))

(event EventTick
  (params (DeltaSeconds :type Float%20%28single-precision%29)))

(event EventInteractwith
  (params (Character :type Character%20Object%20Reference))
  (|CallParentFunction Character))

(event EventPickUp
  (params (CanAddd? :type Boolean) (ParentActor :type Actor%20Object%20Reference) (SocketName :type Name))
  (if CanAddd?
    (bind _aspinn_bp (Utilities|Casting|CastToPinn_Bp ParentActor)
      (:then
        (Default|AddItem (Variables|/Game/PinnBP/Pinn_Bp.Pinn_Bp_C|GetInventory _aspinn_bp) self))
      (:CastFailed
        _))
    (CallFunction|Interactwith _aspinn_bp)
    (Actor|DestroyActor)))

(fn ConstructionScript
  (|CallParentFunction)
  (Rendering|Components|Sprite|SetSprite (Variables|Default|GetBillboard) (Variables|Default|GetIcon)))