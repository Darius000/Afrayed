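; Interactable book actor that tips over when a character hits its collision box.
; The Box hit event calls InteractWith, which runs the parent behavior and then plays a timeline.
; The timeline's Alpha track drives actor pitch directly as an absolute rotation, with roll and yaw forced to zero.
; The construction script calls SetCollisionToComponent with the box and static mesh.
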(event OnComponentHit(Box)
  (params (HitComponent :type Primitive%20Component%20Object%20Reference) (OtherActor :type Actor%20Object%20Reference) (OtherComp :type Primitive%20Component%20Object%20Reference) (NormalImpulse :type Vector :default "0, 0, 0") (Hit :type Hit%20Result%20Structure%20%28by%20ref%29))
  (bind _ascharacter (Utilities|Casting|CastToCharacter OtherActor))
  (CallFunction|Interactwith _ascharacter))

(event EventBeginPlay)

(event Collision|EventActorBeginOverlap
  (params (OtherActor :type Actor%20Object%20Reference)))

(event EventTick
  (params (DeltaSeconds :type Float%20%28single-precision%29)))

(event EventInteractwith
  (params (Character :type Character%20Object%20Reference))
  (|CallParentFunction Character)
  (bind _alpha (Timeline|Timeline_0 Play)
    (:Update
      (Transformation|SetActorRotation (Math|Rotator|MakeRotator 0.0 _alpha 0.0)))))

(fn ConstructionScript
  (CallFunction|SetCollisiontoComponent (Variables|Default|GetBox) (Variables|Default|GetStaticMesh)))