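; InteractableActor is an actor that records whether it has been interacted with.
; The construction script assigns it a new GUID only when the current one is invalid, giving it an identity.
; The Interactwith event sets the InteractedWith flag, and WasInteractedWith returns that flag together with the GUID as the actor ID.
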(event EventBeginPlay)

(event Collision|EventActorBeginOverlap
  (params (OtherActor :type Actor%20Object%20Reference)))

(event EventInteractwith
  (params (Character :type Character%20Object%20Reference))
  (Variables|Interact|SetInteractedWith true))

(event EventTick
  (params (DeltaSeconds :type Float%20%28single-precision%29)))

(fn ConstructionScript
  ;[1 1 1] generates a new GUID for this actor
  (if (not (Guid|IsValidGuid (Variables|ID|GetGUID)))
    (Variables|ID|SetGUID (Guid|NewGuid))))

(fn WasInteractedWith?
  (return (Variables|ID|GetGUID) (Variables|Interact|GetInteractedWith)))