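; Blueprint function library with a helper that resizes a collision shape to match another component's bounds.
; SetCollisionToComponent branches on the exact class of the collision component and updates overlaps after resizing.
; A box takes the bounds' box extent, a sphere takes the sphere radius, and a capsule takes half the Y and Z extents as radius and half-height.
; It changes only size, and other classes are left untouched.
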(fn SetCollisiontoComponent
  (params (CollisionComponent :type Scene%20Component%20Object%20Reference) (Component :type Scene%20Component%20Object%20Reference))
  (bind _returnvalue (Utilities|GetClass CollisionComponent))
  (bind (_origin _boxextent _sphereradius) (Collision|GetComponentBounds Component))
  (bind (_x _y _z) (Math|Vector|BreakVector _boxextent))
  (LocalVariables|SetLocalSceneComponent CollisionComponent)
  (if (== _returnvalue "/Script/Engine.BoxComponent")
    (bind _asbox_collision (Utilities|Casting|CastToBoxComponent (LocalVariables|GetLocalSceneComponent)))
    (Components|Box|SetBoxExtent _asbox_collision _boxextent true)
    (elif (== _returnvalue "/Script/Engine.SphereComponent")
      (bind _assphere_collision (Utilities|Casting|CastToSphereComponent (LocalVariables|GetLocalSceneComponent)))
      (Components|Sphere|SetSphereRadius _assphere_collision _sphereradius true)
      (elif (== _returnvalue "/Script/Engine.CapsuleComponent")
        (bind _ascapsule_collision (Utilities|Casting|CastToCapsuleComponent (LocalVariables|GetLocalSceneComponent)))
        (Components|Capsule|SetCapsuleSize _ascapsule_collision (/ _y 2.0) (/ _z 2.0) true)))))