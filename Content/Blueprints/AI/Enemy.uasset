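; Enemy character that walks a chain of target points under AI control and can be damaged and killed.
; When FollowPath is set, BeginPlay sets the walk speed and writes alive state and start location to the Blackboard.
; Capsule overlaps with EnemyTarget actors pass each one's next point to the Blackboard.
; Damage records the causer and feeds HealthComponent, whose death event blends in mesh physics and clears the alive flag.
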(event OnComponentBeginOverlap(CapsuleComponent)
  (params (OverlappedComponent :type Primitive%20Component%20Object%20Reference) (OtherActor :type Actor%20Object%20Reference) (OtherComp :type Primitive%20Component%20Object%20Reference) (OtherBodyIndex :type Integer) (bFromSweep :type Boolean) (SweepResult :type Hit%20Result%20Structure%20%28by%20ref%29))
  (bind _asenemy_target (Utilities|Casting|CastToEnemyTarget OtherActor))
  (CallFunction|SetNextLocation "TargetLocation" (Transformation|GetActorLocation (Variables|/Game/Blueprints/AI/EnemyTarget.EnemyTarget_C|GetNextTargetPoint _asenemy_target))))

(event OnDeath(HealthComponent)
  (Class|SkeletalMeshComponent|SetPhysicsBlendWeight (Variables|Character|GetMesh) 1.0)
  (CallFunction|SetAlive "Alive" false))

(event EventBeginPlay
  (if (Variables|AI|Traveling|GetFollowPath)
    (CallFunction|SetAlive "Alive" true)
    (CallFunction|SetNextLocation "TargetLocation" (Transformation|GetActorLocation (Variables|AI|Traveling|GetStartLocation)))
    (Variables|/Script/Engine.CharacterMovementComponent|SetMaxWalkSpeed (Variables|Character|GetCharacterMovement) 3e+02)))

(event EventDamage
  (params (Damage :type Integer) (Instigator :type Controller%20Object%20Reference) (DamageType :type DamageType%20Enum :default "NewEnumerator0") (DamageCauser :type Actor%20Object%20Reference))
  (Variables|AI|SetEnemy DamageCauser)
  (Default|TakeDamage (Variables|Default|GetHealthComponent) Damage))

(fn ConstructionScript)

(fn SetNextLocation
  (params (KeyName :type Name) (VectorValue :type Vector))
  (AI|Components|Blackboard|SetValueasVector (AI|GetBlackboard 0) KeyName VectorValue))

(fn SetAlive
  (params (KeyName :type Name) (BoolValue :type Boolean))
  (AI|Components|Blackboard|SetValueasBool (AI|GetBlackboard 0) KeyName BoolValue))