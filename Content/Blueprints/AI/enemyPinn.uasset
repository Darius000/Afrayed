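; Enemy AI pawn whose SeekPlayer event issues a move toward the Enemy0 actor, with a random navigable point as destination, and re-issues it every two seconds.
; LookFor sphere-traces forward from EyeLocation and returns the first hit's actor and location, but its call sits in unconnected nodes.
; Nothing in this graph starts SeekPlayer from outside its own loop, and the GetDistance helper is unused here.
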(event Custom|Seek%20Player
  (AI|AIMoveTo self (Class|NavigationSystem|GetRandomPointinNavigableRadius (Transformation|GetActorLocation) (Variables|AI|Movement|GetReachableRadius) (Variables|AI|Movement|GetNavMesh) (Variables|AI|Movement|GetFilter)) (Variables|AI|GetEnemy_0) 1e+02 true
    (:then
      _)
    (:OnSuccess
      _)
    (:OnFail
      _))
  (Utilities|FlowControl|Delay 2.0)
  (CallFunction|SeekPlayer))

(event EventTick
  (params (DeltaSeconds :type Float%20%28single-precision%29)))

(fn ConstructionScript)

(fn GetDistance
  (params (Target :type Actor%20Object%20Reference))
  (return (Math|Vector|VectorLength (- (Transformation|GetActorLocation) (Transformation|GetActorLocation Target)))))

(fn Lookfor
  (bind _eyelocation (Variables|Default|GetEyeLocation))
  (bind _returnvalue (Transformation|GetWorldLocation _eyelocation))
  (bind (_outhits _returnvalue_2) (Collision|MultiSphereTraceForObjects _returnvalue (+ _returnvalue (* (Math|Vector|GetForwardVector _eyelocation) (LocalVariables|GetDistance))) (Variables|AI|GetSearchRadius) (Utilities|Array|MakeArray "ObjectTypeQuery1" "ObjectTypeQuery4" "ObjectTypeQuery5" "ObjectTypeQuery6") true 0 "ForOneFrame"))
  (if _returnvalue_2
    (for _array_element _outhits
      (return (.Location (Collision|BreakHitResult _array_element)) (.HitActor (Collision|BreakHitResult _array_element))))
    (else
      (return "0, 0, 0" 0))))