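; Actor component that holds an inventory as an array of slot structs, storing each picked-up item's class and icon rather than the actor.
; AddItem fills the first empty slot, and removal by index or current item clears one, each firing a dispatcher with the slot index.
; UseItem spawns the stored class at zero scale on the owner, calls UseMessage, then clears the slot.
; SetCurrentItemIndex is an empty stub.
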(event EventBeginPlay)

(event EventTick
  (params (DeltaSeconds :type Float%20%28single-precision%29)))

(fn AddItem
  (params (PickableActor :type Pickable%20Actor%20Object%20Reference))
  (LocalVariables|SetLocActor PickableActor)
  (bind (_array_element _array_index) (Utilities|Array|ForEachLoopwithBreak (Variables|InventoryData|GetInventoryList) :!label _label)
    (:LoopBody
      (if (not (.isset _array_element))
        (LocalVariables|SetLocIndex _array_index)
        (goto _label Break)))
    (:Completed
      (Utilities|Array|SetArrayElem (Variables|InventoryData|GetInventoryList) (LocalVariables|GetLocIndex) (Utilities|Struct|MakeInventoryData true (Utilities|GetClass (LocalVariables|GetLocActor)) 1 1 (Variables|/Game/Blueprints/Interactables/PickableActor.PickableActor_C|GetIcon (LocalVariables|GetLocActor))))
      (Default|CallOnAddItem (LocalVariables|GetLocIndex)))))

(fn RemoveItem
  (params (Index :type Integer))
  (LocalVariables|SetLocIndex Index)
  (Default|CallOnRemoveItem (.class (Utilities|Array|Get(acopy) (Variables|InventoryData|GetInventoryList) (LocalVariables|GetLocIndex))) (LocalVariables|GetLocIndex))
  (Utilities|Array|SetArrayElem (Variables|InventoryData|GetInventoryList) (LocalVariables|GetLocIndex) (Utilities|Struct|MakeInventoryData false 0 0 0)))

(fn GetSize
  (bind _inventorylist (Variables|InventoryData|GetInventoryList))
  (return (Utilities|Array|Length _inventorylist) _inventorylist))

(fn RemoveCurrentItem
  (LocalVariables|SetLocIndex (Variables|Default|GetCurrentItem))
  (Default|CallOnRemoveItem (.Class (Utilities|Struct|BreakInventoryData (Utilities|Array|Get(acopy) (Variables|InventoryData|GetInventoryList) (LocalVariables|GetLocIndex)))) (LocalVariables|GetLocIndex))
  (Utilities|Array|SetArrayElem (Variables|InventoryData|GetInventoryList) (LocalVariables|GetLocIndex) (Utilities|Struct|MakeInventoryData false))
  (return))

(fn HaveSpace
  (bind _array_element (Utilities|Array|ForEachLoopwithBreak (Variables|InventoryData|GetInventoryList) :!label _label)
    (:LoopBody
      (if (.IsSet (Utilities|Struct|BreakInventoryData _array_element))
        (LocalVariables|SetHasSpace? false)
        (else
          (LocalVariables|SetHasSpace? true)
          (goto _label Break))))
    (:Completed
      (return (LocalVariables|GetHasSpace?)))))

(fn SetCurrentItemIndex)

(fn GetItematAindex
  (params (Index :type Integer))
  (return (Utilities|Array|Get(acopy) (Variables|InventoryData|GetInventoryList) Index)))

(fn UseItem
  (params (Index :type Integer))
  (LocalVariables|SetLocIndex Index)
  (bind _returnvalue (Game|SpawnActorfromClass (.class (Utilities|Array|Get(acopy) (Variables|InventoryData|GetInventoryList) (LocalVariables|GetLocIndex))) (Math|Transform|MakeTransform (Transformation|GetActorLocation (Components|GetOwner)) "0, 0, 0" "0.000000,0.000000,0.000000") "AlwaysSpawn" 0 0))
  (Class|InteractionsInterafce|Use(Message) _returnvalue)
  (Utilities|Array|SetArrayElem (Variables|InventoryData|GetInventoryList) (LocalVariables|GetLocIndex) (Utilities|Struct|MakeInventoryData false)))