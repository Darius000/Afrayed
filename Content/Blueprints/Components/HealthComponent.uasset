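; Health component that tracks an owner's current and maximum health and handles damage, healing and death.
; TakeDamage subtracts from Health while it is above zero, fires the receive-damage event, sets Dead and fires the death event at zero or below, and returns Dead.
; RestoreHealth adds a clamped amount when below MaxHealth and fires a restore event.
; GetHealth exposes both health values.
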(fn TakeDamage
  (params (Damage :type Integer))
  (if (> (Variables|Default|GetHealth) 0)
    (bind _output_get (Variables|Default|SetHealth (- (Variables|Default|GetHealth) Damage)))
    (Default|CallOnRecieveDamage)
    (if (<= _output_get 0)
      (Variables|Default|SetDead true)
      (Default|CallOnDeath))
    (return (Variables|Default|GetDead))
    (else
      (return (Variables|Default|GetDead)))))

(fn GetHealth
  (return (Variables|Default|GetHealth) (Variables|Default|GetMaxHealth)))

(fn RestoreHealth
  (params (Amount :type Integer))
  (if (< (Variables|Default|GetHealth) (Variables|Default|GetMaxHealth))
    (Variables|Default|SetHealth (+ (Variables|Default|GetHealth) (Math|Integer|Clamp(Integer) Amount Amount (- (Variables|Default|GetMaxHealth) (Variables|Default|GetHealth)))))
    (Default|CallOnRestoreHealth)
    (return)
    (else
      (return))))