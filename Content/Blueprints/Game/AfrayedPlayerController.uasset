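; Player controller for the Pinn character, handling movement, jumping, running, camera look and the pause menu.
; It caches the possessed Pinn_Bp on BeginPlay and forwards input to it, blocking movement actions when Dead and allowing jumps only while Walking or Running.
; Movement follows the spring arm's axes, and Run switches max walk speed.
; A FlipFlop on PauseGame toggles game pause, the PauseMenu widget, cursor and input mode.
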(event EventBeginPlay
  ;[0.175 0.175 0.175] Get Controlled Pawn
  (bind _aspinn_bp (Utilities|Casting|CastToPinn_Bp (Pawn|GetControlledPawn)))
  (Variables|Pawn|SetPinnPawn _aspinn_bp))

(event Input|ActionEvents|InputActionJump
  (params (Key :type Key%20Structure :default "AnyKey"))
  (bind _characterstate (CallFunction|GetPinnState))
  ;[0.07 0.07 0.07] Character Movement
  (:Pressed
    (if (Utilities|Enum|NotEqual(Enum) _characterstate "NewEnumerator4")
      (switch Utilities|FlowControl|Switch|SwitchonPinnCharacterState _characterstate
        (:NewEnumerator0
          _)
        (:NewEnumerator2
          _))
      (Character|Jump (Variables|Pawn|GetPinnPawn)))))

(event Input|ActionEvents|InputActionRun
  (params (Key :type Key%20Structure :default "AnyKey"))
  (bind _characterstate (CallFunction|GetPinnState))
  (bind _pinnpawn (Variables|Pawn|GetPinnPawn))
  (bind _returnvalue (Utilities|Enum|NotEqual(Enum) _characterstate "NewEnumerator4"))
  (bind _charactermovement (Variables|/Script/Engine.Character|GetCharacterMovement _pinnpawn))
  ;[0.07 0.07 0.07] Character Movement
  (:Pressed
    (if _returnvalue
      (Variables|/Script/Engine.CharacterMovementComponent|SetMaxWalkSpeed _charactermovement 6e+02)))
  (:Released
    (if _returnvalue
      (Variables|/Script/Engine.CharacterMovementComponent|SetMaxWalkSpeed _charactermovement 3e+02))))

(event Input|ActionEvents|InputActionPauseGame
  (params (Key :type Key%20Structure :default "AnyKey"))
  ;[0.075 0.075 0.075] Pausing
  (:Pressed
    (Utilities|FlowControl|FlipFlop
      (:A
        (Game|SetGamePaused true)
        (bind _returnvalue (UserInterface|CreateWidget "/Game/UI/PauseMenu.PauseMenu_C"))
        (bind _output_get (Variables|Default|SetPauseWidget _returnvalue))
        (UserInterface|Viewport|AddtoViewport _output_get 0)
        (Input|SetInputModeUIOnly 0 (Variables|Default|GetPauseWidget) "DoNotLock")
        (Variables|Default|SetbShowMouseCursor true))
      (:B
        (Game|SetGamePaused false)
        (Variables|Default|SetbShowMouseCursor false)
        (Input|SetInputModeGameOnly)
        (Widget|RemovefromParent (Variables|Default|GetPauseWidget))))))

(event Input|AxisEvents|InputAxisMoveForward
  (params (AxisValue :type Float%20%28single-precision%29))
  ;[0.07 0.07 0.07] Character Movement
  (if (Utilities|Enum|NotEqual(Enum) (CallFunction|GetPinnState) "NewEnumerator4")
    (Class|PawnMovementComponent|AddInputVector (Variables|/Script/Engine.Character|GetCharacterMovement (Variables|Pawn|GetPinnPawn)) (* (Math|Vector|GetForwardVector (Variables|/Game/PinnBP/Pinn_Bp.Pinn_Bp_C|GetSpringArm (Variables|Pawn|GetPinnPawn))) AxisValue) false)))

(event Input|AxisEvents|InputAxisMoveRight
  (params (AxisValue :type Float%20%28single-precision%29))
  ;[0.07 0.07 0.07] Character Movement
  (if (Utilities|Enum|NotEqual(Enum) (CallFunction|GetPinnState) "NewEnumerator4")
    (Class|PawnMovementComponent|AddInputVector (Variables|/Script/Engine.Character|GetCharacterMovement (Variables|Pawn|GetPinnPawn)) (* (Math|Vector|GetRightVector (Variables|/Game/PinnBP/Pinn_Bp.Pinn_Bp_C|GetSpringArm (Variables|Pawn|GetPinnPawn))) AxisValue) false)))

(event Input|AxisEvents|InputAxisTurn
  (params (AxisValue :type Float%20%28single-precision%29))
  ;[0.07 0.07 0.07] Character Movement
  (Pawn|Input|AddControllerYawInput (Variables|Pawn|GetPinnPawn) (* AxisValue (Variables|Camera|GetCameraRate))))

(event Input|AxisEvents|InputAxisLookUp
  (params (AxisValue :type Float%20%28single-precision%29))
  ;[0.07 0.07 0.07] Character Movement
  (Pawn|Input|AddControllerPitchInput (Variables|Pawn|GetPinnPawn) (* AxisValue (Variables|Camera|GetCameraRate))))

(fn ConstructionScript)

(fn GetPinnState
  (return (Variables|/Game/PinnBP/Pinn_Bp.Pinn_Bp_C|GetCharacterState (Variables|Pawn|GetPinnPawn))))