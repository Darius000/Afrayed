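; Player character Blueprint for Pinn, with enemy lock-on, melee combos and an aimable needle-thread cable.
; Lock-on gathers enemies within range, picks the one closest to the camera's yaw, and can cycle targets.
; While locked, Tick interpolates the spring arm toward the target and snaps actor yaw to face it.
; Attack plays or continues the combo montage, or extends the cable when aiming; needle capsule overlaps apply damage.
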(event OnComponentBeginOverlap(Needle_Hit_Capsule)
  (params (OverlappedComponent :type Primitive%20Component%20Object%20Reference) (OtherActor :type Actor%20Object%20Reference) (OtherComp :type Primitive%20Component%20Object%20Reference) (OtherBodyIndex :type Integer) (bFromSweep :type Boolean) (SweepResult :type Hit%20Result%20Structure%20%28by%20ref%29))
  ;[1 1 1] Takes Damage
  (Game|Damage|ApplyDamage OtherActor (Variables|Default|GetAttackPower) 0 self))

(event Custom|LockOn
  (if (Variables|Default|GetIsLookedOn)
    (CallFunction|LockOff)
    (else
      ;[1 1 1] Lock On
      (Variables|Default|SetIsLookedOn true)
      (Variables|Default|SetCameraRate 0.0)
      (bind _outactors (Actor|GetAllActorsOfClass "/Game/Blueprints/Enemy.Enemy_C"))
      (for _array_element _outactors
        (if (< (CallFunction|GetEnemyDistance _array_element) (Variables|Default|GetMaxLockDistance))
          (Utilities|Array|Add (Variables|Default|GetLockList) _array_element)
          (Development|PrintString (Utilities|GetDisplayName _array_element))
          (if (.IsLeast (CallFunction|FindRotationDistance (Variables|Default|GetCamera) (Variables|Default|GetSpringArm) _array_element))
            (Variables|Default|SetMaxLockRotation (.Yaw (CallFunction|FindRotationDistance (Variables|Default|GetCamera) (Variables|Default|GetSpringArm) _array_element)))
            (bind _output_get (Variables|Default|SetEnemy _array_element))
            (Development|PrintString (Utilities|String|Append "Target is:" (Utilities|GetDisplayName _output_get))))))
      (if (!= (Variables|Default|GetEnemy) 0)
        (Variables|/Script/Engine.SpringArmComponent|SetbUsePawnControlRotation (Variables|Default|GetSpringArm) false)
        (else
          (CallFunction|LockOff))))))

(event Custom|LockOff
  ;[1 1 1] Used for Resetting Camera
  (Pawn|SetControlRotation (Pawn|GetController) (CallFunction|GetNewRotation))
  (Variables|Default|SetIsLookedOn false)
  (Variables|Default|SetEnemy 0)
  (Variables|/Script/Engine.SpringArmComponent|SetbUsePawnControlRotation (Variables|Default|GetSpringArm) true)
  (Utilities|Array|Clear (Variables|Default|GetLockList))
  (Variables|Default|SetMaxLockRotation 9e+01))

(event Custom|NextTarget
  ;[1 1 1] Toggle Enemy
  (bind _asenemy (Utilities|Casting|CastToEnemy (Variables|Default|GetEnemy)))
  (Variables|Default|SetLL_current (Utilities|Array|FindItem (Variables|Default|GetLockList) _asenemy))
  (if (>= (Variables|Default|GetLL_current) (- (Utilities|Array|Length (Variables|Default|GetLockList)) 1))
    (Variables|Default|SetLL_current 0)
    (else
      (Math|Integer|IncrementInt (Variables|Default|GetLL_current)
        (:%20%20
          _))))
  (Variables|Default|SetEnemy (Utilities|Array|Get(acopy) (Variables|Default|GetLockList) (Variables|Default|GetLL_current))))

(event EventTick
  (params (DeltaSeconds :type Float%20%28single-precision%29))
  (bind _returnvalue (Transformation|GetActorRotation))
  (bind _maxcamerarate (Variables|Default|GetMaxCameraRate))
  (Variables|Default|SetDeltaTime DeltaSeconds)
  (if (Variables|Default|GetIsLookedOn)
    (Transformation|SetWorldRotation (Variables|Default|GetSpringArm) (CallFunction|GetNewRotation) false false)
    (Transformation|SetActorRotation (Math|Rotator|MakeRotator (.roll _returnvalue) (.pitch _returnvalue) (.yaw (Math|Rotator|FindLookatRotation (Transformation|GetActorLocation) (Transformation|GetActorLocation (Variables|Default|GetEnemy))))))
    (Development|PrintString (Utilities|String|ToString(Float) (.yaw (Transformation|GetWorldRotation (Variables|Default|GetSpringArm)))))
    (else
      ;[1 1 1] Slow Camera Rate Increase
      (if (< (Variables|Default|GetCameraRate) _maxcamerarate)
        (if (> (+ (* DeltaSeconds 1.0) (Variables|Default|GetCameraRate)) _maxcamerarate)
          (Variables|Default|SetCameraRate 0.5)
          (else
            (Variables|Default|SetCameraRate (+ (* DeltaSeconds 1.0) (Variables|Default|GetCameraRate)))))))))

(event Input|ActionEvents|InputActionAim
  (params (Key :type Key%20Structure :default "AnyKey"))
  ;[1 1 1] Set Aiming and length of cable
  (:Pressed
    (Variables|Default|SetNotAiming false))
  (:Released
    (Variables|Default|SetNotAiming true)
    (Variables|/Script/CableComponent.CableComponent|SetCableLength (Variables|Default|GetNeedleThread) 5e+01)))

(event Input|ActionEvents|InputActionAttack
  (params (Key :type Key%20Structure :default "AnyKey"))
  (bind _mesh (Variables|Character|GetMesh))
  (bind _returnvalue (Components|SkeletalMesh|GetAnimInstance _mesh))
  ;[1 1 1] Combo Attack
  (:Pressed
    (if (Variables|Default|GetNotAiming)
      (if (Variables|Default|GetNotFighting)
        (Variables|Default|SetNotFighting false)
        (bind _returnvalue_2 (Animation|GetCurrentMontage :!class /Script/Engine.Character))
        (if (== _returnvalue_2 "/Game/Pinn/Animation/Pinn_Attack_Montage.Pinn_Attack_Montage")
          (bind _aspinn_anim_bp (Utilities|Casting|CastToPinn_AnimBp _returnvalue))
          (Default|ContinueCombo _aspinn_anim_bp)
          (else
            (Animation|Montage|MontagePlay _returnvalue "/Game/Pinn/Animation/Pinn_Attack_Montage.Pinn_Attack_Montage" 1.0 "MontageLength" 0.0))))
      (else
        (Variables|/Script/CableComponent.CableComponent|SetCableLength (Variables|Default|GetNeedleThread) (Variables|Default|GetRopeMaxLength)))))
  (:Released
    (Variables|Default|SetNotFighting true)))

(event Input|ActionEvents|InputActionToggleLockOn
  (params (Key :type Key%20Structure :default "AnyKey"))
  ;[1 1 1] Lock On
  (:Pressed
    (CallFunction|Lockon)))

(event Input|ActionEvents|InputActionNextTarget
  (params (Key :type Key%20Structure :default "AnyKey"))
  ;[1 1 1] Toggle Enemy
  (:Pressed
    (CallFunction|NextTarget)))

(fn ConstructionScript)

(fn GetEnemyDistance
  (params (Target :type Actor%20Object%20Reference))
  (return (Math|Vector|VectorLength (- (Transformation|GetActorLocation Target) (Transformation|GetActorLocation)))))

(fn GetLookatRotation
  (params (Camera :type Scene%20Component%20Object%20Reference) (Enemy :type Actor%20Object%20Reference))
  (return (Math|Rotator|FindLookatRotation (Transformation|GetWorldLocation Camera) (Transformation|GetActorLocation Enemy))))

(fn FindRotationDistance
  (params (Camera :type Scene%20Component%20Object%20Reference) (Spring%20Arm :type Scene%20Component%20Object%20Reference) (Enemy :type Actor%20Object%20Reference))
  (bind _returnvalue (Transformation|GetWorldRotation Camera))
  (bind _returnvalue_2 (Transformation|GetWorldLocation Spring%20Arm))
  (bind _returnvalue_3 (Transformation|GetActorLocation Enemy))
  (bind _returnvalue_4 (Math|Rotator|FindLookatRotation _returnvalue_2 _returnvalue_3))
  (bind _returnvalue_5 (Math|Float|Absolute(Float) (.yaw _returnvalue)))
  (bind _returnvalue_6 (Math|Float|Absolute(Float) (.yaw _returnvalue_4)))
  (bind _returnvalue_7 (- _returnvalue_6 _returnvalue_5))
  (bind _returnvalue_8 (Math|Float|Absolute(Float) _returnvalue_7))
  (return _returnvalue_8 (< _returnvalue_8 (Variables|Default|GetMaxLockRotation))))

(fn GetNewRotation
  (bind _intspeed (Variables|Default|GetintSpeed))
  (bind _enemy (Variables|Default|GetEnemy))
  (bind _springarm (Variables|Default|GetSpringArm))
  (bind _deltatime (Variables|Default|GetDeltaTime))
  (bind _returnvalue (CallFunction|GetLookatRotation _springarm _enemy))
  (bind _returnvalue_2 (Transformation|GetWorldRotation _springarm))
  (bind (_roll _pitch _yaw) (Math|Rotator|BreakRotator _returnvalue))
  (if (!= _enemy 0)
    (return (Class|KismetMathLibrary|RInterptoConstant _returnvalue_2 (Math|Rotator|MakeRotator _roll _pitch _yaw) _deltatime _intspeed))
    (else
      (return (Class|KismetMathLibrary|RInterptoConstant _returnvalue_2 (Pawn|GetControlRotation :!class /Script/Engine.Pawn) _deltatime _intspeed)))))